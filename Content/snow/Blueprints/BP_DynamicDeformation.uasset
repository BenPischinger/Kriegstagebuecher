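; Dynamic deformable snow plane that records objects within range of an orthographic scene capture and displaces a tessellated surface.
; A depth-limited post-process feeds the capture target, drawn each tick into a persistent render target through a masked or additive material, which drives displacement.
; Optional regeneration additively draws four randomly placed dots per tick to build up recovery.
; The construction script creates targets on demand, per-instance materials, and matched plane and capture scaling.
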(event `self.ReceiveTick`
  (params (DeltaSeconds :type "Float (single-precision)"))
  (bind _dotmat (`self.DotMat`))
  (if (`self.Additive or Masked`)
    ;[1 1 1] Main part of the function, draws the camera view to a render target
    (`KismetRenderingLibrary.DrawMaterialToRenderTarget` (`self.Render`) (`self.MaterialTargetAdditive`))
    (else
      (`KismetRenderingLibrary.DrawMaterialToRenderTarget` (`self.Render`) (`self.MaterialTarget`))))
  ;[1 1 1] allows you to toggle regeneration
  (if (`self.Regeneration`)
    ;[1 1 1] used for regeneration, the material has 4 spots and at every tick they are assigned to a different location and then drawn to the render target with an additive material, which creates the buildup effect
    (`MaterialInstanceDynamic.SetScalarParameterValue` _dotmat "RandX" (`KismetMathLibrary.RandomFloatInRange` 0.0 1.0))
    (`MaterialInstanceDynamic.SetScalarParameterValue` _dotmat "RandY" (`KismetMathLibrary.RandomFloatInRange` 0.0 1.0))
    (`MaterialInstanceDynamic.SetScalarParameterValue` _dotmat "RandX2" (`KismetMathLibrary.RandomFloatInRange` 0.0 1.0))
    (`MaterialInstanceDynamic.SetScalarParameterValue` _dotmat "RandY2" (`KismetMathLibrary.RandomFloatInRange` 0.0 1.0))
    (`MaterialInstanceDynamic.SetScalarParameterValue` _dotmat "RandX3" (`KismetMathLibrary.RandomFloatInRange` 0.0 1.0))
    (`MaterialInstanceDynamic.SetScalarParameterValue` _dotmat "RandY3" (`KismetMathLibrary.RandomFloatInRange` 0.0 1.0))
    (`MaterialInstanceDynamic.SetScalarParameterValue` _dotmat "RandX4" (`KismetMathLibrary.RandomFloatInRange` 0.0 1.0))
    (`MaterialInstanceDynamic.SetScalarParameterValue` _dotmat "RandY4" (`KismetMathLibrary.RandomFloatInRange` 0.0 1.0))
    (`KismetRenderingLibrary.DrawMaterialToRenderTarget` (`self.Render`) _dotmat)))

(event `self.ReceiveBeginPlay`
  (bind _render (`self.Render`))
  ;[1 1 1] somehow required, without it it doesn't clear the targets properly
  (`KismetSystemLibrary.Delay` 0.05)
  ;[1 1 1] clears the render target so you can specify whether you want it to start with snow, i used a delay because it didn't work otherwise
  (if (`self.Start with Snow`)
    (`KismetRenderingLibrary.ClearRenderTarget2D` _render)
    (else
      (`KismetRenderingLibrary.ClearRenderTarget2D` _render (struct :`R` 1.0 :`G` 1.0 :`B` 1.0 :`A` 1.0)))))

(fn `UserConstructionScript`
  (bind _scale (`self.Scale`))
  (bind _texturesize (`self.TextureSize`))
  (bind _capture (`self.Capture`))
  (bind _capture_2 (`self.Capture`))
  (bind _render (`self.Render`))
  (bind _returnvalue (* 1.0 _scale))
  (bind _returnvalue_2 (`KismetMathLibrary.MakeVector` _returnvalue _returnvalue 1.0))
  ;[1 1 1] Toggles Visibility on the simple plane to give you the option of two different effects
  (`SceneComponent.SetVisibility` (`self.Geometry_Simple`) (`self.Toggle Setup Type`) false)
  (if (`self.Reload Textures`)
    ;[1 1 1] Create render targets (due to a bug it must be done like this)
    (bind _returnvalue_3 (`KismetRenderingLibrary.CreateRenderTarget2D` _texturesize _texturesize))
    (set `self.Capture` _returnvalue_3)
    (bind _returnvalue_4 (`KismetRenderingLibrary.CreateRenderTarget2D` _texturesize _texturesize))
    (set `self.Render` _returnvalue_4)
    ;[1 1 1] Clamping Render Targets without this the border of the texture doesn't get effected
    (set `TextureRenderTarget2D.AddressX` "TA_Clamp" _capture_2)
    (set `TextureRenderTarget2D.AddressY` "TA_Clamp" _capture_2)
    (set `TextureRenderTarget2D.AddressX` "TA_Clamp" _render)
    (set `TextureRenderTarget2D.AddressY` "TA_Clamp" _render)
    (set `self.Reload Textures` false))
  ;[1 1 1] Create dynamic material instance of the tessellated plane material and apply
  (bind _returnvalue_5 (`KismetMaterialLibrary.CreateDynamicMaterialInstance` (`self.Tessellation Material`)))
  (bind _output_get (set `self.Tess_Dynamic_Material` _returnvalue_5))
  (`PrimitiveComponent.SetMaterial` (`self.Geometry_Tessellated Plane`) 0 _output_get)
  ;[1 1 1] set material to simple plane
  (`PrimitiveComponent.SetMaterial` (`self.Geometry_Simple`) 0 (`self.Simple Plane Material`))
  ;[1 1 1] Dynamic Material instances so the blueprint can be duplicated
  (bind _returnvalue_6 (`KismetMaterialLibrary.CreateDynamicMaterialInstance` "/Game/snow/Materials/Mat_MaterialTargetforRenderMasked_Inst.Mat_MaterialTargetforRenderMasked_Inst"))
  (set `self.MaterialTarget` _returnvalue_6)
  (bind _returnvalue_7 (`KismetMaterialLibrary.CreateDynamicMaterialInstance` "/Game/snow/Materials/Mat_MaterialTargetforRenderAdditive_Inst.Mat_MaterialTargetforRenderAdditive_Inst"))
  (set `self.MaterialTargetAdditive` _returnvalue_7)
  (bind _returnvalue_8 (`KismetMaterialLibrary.CreateDynamicMaterialInstance` "/Game/snow/Materials/Mat_BlendableforCapture2dPost_Inst2.Mat_BlendableforCapture2dPost_Inst2"))
  (set `self.PostprocessCameraMat` _returnvalue_8)
  (bind _returnvalue_9 (`KismetMaterialLibrary.CreateDynamicMaterialInstance` "/Game/snow/Materials/Mat_recovermat_Inst.Mat_recovermat_Inst"))
  (set `self.DotMat` _returnvalue_9)
  ;[1 1 1] Add render targets to dynamic material instances
  (`MaterialInstanceDynamic.SetTextureParameterValue` (`self.Tess_Dynamic_Material`) "Param_R2d" (`self.Render`))
  (`MaterialInstanceDynamic.SetTextureParameterValue` (`self.MaterialTarget`) "Param_scenecap" _capture)
  (`MaterialInstanceDynamic.SetTextureParameterValue` (`self.MaterialTargetAdditive`) "Param_scenecap" _capture)
  ;[1 1 1] Adds Render Target to Scene Capture
  (set `SceneCaptureComponent2D.TextureTarget` (`self.Capture`) (`self.SceneCaptureComponent2D`))
  ;[1 1 1] Scales the plane and the camera view width at the same time
  (`SceneComponent.SetWorldScale3D` (`self.Geometry_Tessellated Plane`) _returnvalue_2)
  (`SceneComponent.SetWorldScale3D` (`self.Geometry_Simple`) _returnvalue_2)
  (set `SceneCaptureComponent2D.OrthoWidth` (* 1000.0 _scale) (`self.SceneCaptureComponent2D`))
  ;[1 1 1] Material Displacement Values
  (`MaterialInstanceDynamic.SetScalarParameterValue` (`self.Tess_Dynamic_Material`) "3_Dynamic Deformation Down" (`self.Displacement Down`))
  (`MaterialInstanceDynamic.SetScalarParameterValue` (`self.Tess_Dynamic_Material`) "2_Displacement Up" (`self.Displace Up`))
  (`MaterialInstanceDynamic.SetScalarParameterValue` (`self.Tess_Dynamic_Material`) "4_Tess Multi" (`self.Tessellation Multiply`))
  ;[1 1 1] Regeneration
  (`MaterialInstanceDynamic.SetScalarParameterValue` (`self.DotMat`) "Density(edit using blueprint)" (`self.Regen Amount`))
  (`MaterialInstanceDynamic.SetScalarParameterValue` (`self.DotMat`) "Radius(edit using blueprint)" (`self.Regen Size`))
  ;[1 1 1] Changes the view distance (camera range)
  (`MaterialInstanceDynamic.SetScalarParameterValue` (`self.PostprocessCameraMat`) "DepthDistance(edit using blueprint)" (`self.CameraVisDistance`))
  (`SceneComponent.K2_SetRelativeTransform` (`self.SceneCaptureComponent2D`) (`KismetMathLibrary.MakeTransform` (`KismetMathLibrary.MakeVector` 0.0 0.0 (`self.Camera Offset`)) (struct :`Pitch` 90.0 :`Roll` -180.0)) false false)
  ;[1 1 1] Adds Blendable Material to scene capture
  (`SceneCaptureComponent2D.AddOrUpdateBlendable` (`self.SceneCaptureComponent2D`) (`self.PostprocessCameraMat`) 1.0)
  ;[1 1 1] used to remove some of the tessellated plane flickering
  (`PrimitiveComponent.SetBoundsScale` (`self.Geometry_Tessellated Plane`) (`self.Bounds Scale (flickering)`))
  ;[1 1 1] this isn't required as the camera can't see the plane but i left it here in case someone wanted to use a two sided material on the tessellated plane
  (bind _outactorlist (`KismetSystemLibrary.GetActorListFromComponentList` (`|MakeArray` (`self.Geometry_Tessellated Plane`) :!type "PrimitiveComponent Object Reference")))
  (set `SceneCaptureComponent.HiddenActors` _outactorlist (`self.SceneCaptureComponent2D`)))