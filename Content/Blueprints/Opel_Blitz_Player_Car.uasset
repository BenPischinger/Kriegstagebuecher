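; Opel Blitz truck actor that plays a scripted ride toward a fixed world position when play begins.
; A timeline moves it in X and Y via FInterpTo, feeding its curve tracks in as DeltaTime, while keeping height unchanged.
; Tick spins the front and rear wheel components by the timeline's BlitzSpeed value.
; Delayed door-opening logic with a Doors timeline is present but disconnected, so it never runs.
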(event `self.ReceiveBeginPlay`
  ;[1 1 1] Truck Ride
  (`|ExecutionSequence`
    (:`then_0`
      (bind (_direction _newtrack_0 _newtrack_1 _blitzspeed) (`Timeline|Timeline_0` :!via `PlayFromStart`)
        (:`Update`
          (`self.K2_SetActorLocation` (`KismetMathLibrary.MakeVector` (`KismetMathLibrary.FInterpTo` (.x (`self.K2_GetActorLocation`)) 233.0 _newtrack_1 0.1) (`KismetMathLibrary.FInterpTo` (.y (`self.K2_GetActorLocation`)) -1514.0 _newtrack_0 0.1) (.z (`self.K2_GetActorLocation`)))))))))

(event `self.ReceiveTick`
  (params (DeltaSeconds :type "Float (single-precision)"))
  ;[1 1 1] Reifen Animation
  (bind _returnvalue (`KismetMathLibrary.MakeRotator` (stale `self.ReceiveBeginPlay` _blitzspeed)))
  (`SceneComponent.K2_AddRelativeRotation` (`self.Opel_Blitz_Rad_Vorn`) _returnvalue false false)
  (`SceneComponent.K2_AddRelativeRotation` (`self.Opel_Blitz_Rad_Hinten`) _returnvalue false false))

(fn `UserConstructionScript`)