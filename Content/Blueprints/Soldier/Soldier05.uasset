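; Soldier05 is a scripted soldier actor that plays a fixed, timed animation sequence when play begins.
; It plays the one-shot Ausstieg_01 (exit) animation, then after a delay sets only its height to the HightAdjustment variable.
; After a much longer delay it jumps to a hardcoded location and rotation and plays Attack_04 once.
; All timing comes from chained Delays, with no AI or external triggers.
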(event `self.ReceiveBeginPlay`
  (`SkeletalMeshComponent.PlayAnimation` (`self.SkeletalMeshComponent`) "/Game/Assets/Character/Soldier_01/Animation/Aussteigen/ausstieg_01.ausstieg_01" false)
  (`KismetSystemLibrary.Delay` 12.5)
  (`self.K2_SetActorLocation` (`KismetMathLibrary.MakeVector` (.x (`self.K2_GetActorLocation`)) (.y (`self.K2_GetActorLocation`)) (`self.HightAdjustment`)))
  (`KismetSystemLibrary.Delay` 90.0)
  (`self.K2_SetActorLocationAndRotation` (626.0 -186.0 -36.0) (struct :`Yaw` 35.0))
  (`SkeletalMeshComponent.PlayAnimation` (`self.SkeletalMeshComponent`) "/Game/Assets/Character/Soldier_01/Animation/Attack/attack_04.attack_04" false))

(fn `UserConstructionScript`)