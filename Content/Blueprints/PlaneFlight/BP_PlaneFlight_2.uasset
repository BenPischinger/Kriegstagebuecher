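; BP_PlaneFlight_2 animates a BF109E42 plane along a scripted flight path using timelines.
; On BeginPlay it sets the plane's starting relative location, then waits on a long delay.
; PlaneRotator then yaws the Rotationpoint component while PlaneLocation drives the plane's relative X and Z.
; Each PlaneLocation update also calls Play on PlaneRotation, which drives the plane's pitch.
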(event `self.ReceiveBeginPlay`
  (`SceneComponent.K2_SetRelativeLocation` (`self.BF-109E4_2`) (`KismetMathLibrary.MakeVector` 100.0 100.0 -200.0) false false)
  (`KismetSystemLibrary.Delay` 80.0)
  (`|ExecutionSequence`
    (:`then_0`
      (bind (_direction _rot_z) (`Timeline|PlaneRotator`)
        (:`Update`
          (`SceneComponent.K2_SetRelativeRotation` (`self.rotationpoint`) (`KismetMathLibrary.MakeRotator` 0.0 0.0 _rot_z) false false))))
    (:`then_1`
      (bind (_direction_2 _loc_x _loc_z) (`Timeline|PlaneLocation`)
        (:`Update`
          (`SceneComponent.K2_SetRelativeLocation` (`self.BF-109E4_2`) (`KismetMathLibrary.MakeVector` _loc_x 0.0 _loc_z) false false)
          (bind (_direction_3 _rot_y) (`Timeline|PlaneRotation`)
            (:`Update`
              (`SceneComponent.K2_SetRelativeRotation` (`self.BF-109E4_2`) (`KismetMathLibrary.MakeRotator` 0.0 _rot_y) false false))))))))

(fn `UserConstructionScript`)