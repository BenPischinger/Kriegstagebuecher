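; PlaneGroundFire actor that plays repeating volleys of explosion particles and sounds, apparently a plane's fire hitting the ground.
; BeginPlay waits 84 seconds, then a Sequence runs two Delay chains offset by 0.05 seconds, activating particle and audio pairs in a rapid interleaved burst.
; Both chains feed a shared 17.5-second Delay that repeats the volley indefinitely.
; The overlap, construction and component activation events are empty.
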(event `self.Blueprint_Effect_Explosion.OnComponentActivated`
  (params (Component :type "ActorComponent Object Reference") (bReset :type Boolean)))

(event `self.Blueprint_Effect_Explosion.OnComponentDeactivated`
  (params (Component :type "ActorComponent Object Reference")))

(event `self.ReceiveBeginPlay`
  (`KismetSystemLibrary.Delay` 84.0)
  (`|ExecutionSequence`
    (:`then_0`
      (`ActorComponent.Activate` (`self.ParticleSystem`) false)
      (`ActorComponent.Activate` (`self.Audio`) false)
      (`KismetSystemLibrary.Delay` 0.1)
      (`ActorComponent.Activate` (`self.P_Explosion02`) false)
      (`ActorComponent.Activate` (`self.S_Explosion02`) false)
      (`KismetSystemLibrary.Delay` 0.1)
      (`ActorComponent.Activate` (`self.P_Explosion03`) false)
      (`ActorComponent.Activate` (`self.S_Explosion03`) false)
      (`KismetSystemLibrary.Delay` 0.1)
      (`ActorComponent.Activate` (`self.Audio3`) false)
      (`ActorComponent.Activate` (`self.ParticleSystem3`) false)
      (`KismetSystemLibrary.Delay` 0.1)
      (`ActorComponent.Activate` (`self.P_Explosion05`) false)
      (`ActorComponent.Activate` (`self.S_Explosion05`) false)
      (`KismetSystemLibrary.Delay` 0.1)
      (`ActorComponent.Activate` (`self.ParticleSystem5`) false)
      (`ActorComponent.Activate` (`self.Audio5`) false))
    (:`then_1`
      (`KismetSystemLibrary.Delay` 0.05)
      (`ActorComponent.Activate` (`self.P_Explosion01`) false)
      (`ActorComponent.Activate` (`self.S_Explosion01`) false)
      (`KismetSystemLibrary.Delay` 0.1)
      (`ActorComponent.Activate` (`self.Audio1`) false)
      (`ActorComponent.Activate` (`self.ParticleSystem1`) false)
      (`KismetSystemLibrary.Delay` 0.1)
      (`ActorComponent.Activate` (`self.ParticleSystem2`) false)
      (`ActorComponent.Activate` (`self.Audio2`) false)
      (`KismetSystemLibrary.Delay` 0.1)
      (`ActorComponent.Activate` (`self.P_Explosion04`) false)
      (`ActorComponent.Activate` (`self.S_Explosion04`) false)
      (`KismetSystemLibrary.Delay` 0.1)
      (`ActorComponent.Activate` (`self.Audio4`) false)
      (`ActorComponent.Activate` (`self.ParticleSystem4`) false)
      (`KismetSystemLibrary.Delay` 0.1)
      (`ActorComponent.Activate` (`self.P_Explosion06`) false)
      (`ActorComponent.Activate` (`self.S_Explosion06`) false)))
  (`KismetSystemLibrary.Delay` 17.5 :!label _label)
  (`|ExecutionSequence`
    (:`then_0`
      (`ActorComponent.Activate` (`self.ParticleSystem`) false)
      (`ActorComponent.Activate` (`self.Audio`) false)
      (`KismetSystemLibrary.Delay` 0.1)
      (`ActorComponent.Activate` (`self.P_Explosion02`) false)
      (`ActorComponent.Activate` (`self.S_Explosion02`) false)
      (`KismetSystemLibrary.Delay` 0.1)
      (`ActorComponent.Activate` (`self.P_Explosion03`) false)
      (`ActorComponent.Activate` (`self.S_Explosion03`) false)
      (`KismetSystemLibrary.Delay` 0.1)
      (`ActorComponent.Activate` (`self.Audio3`) false)
      (`ActorComponent.Activate` (`self.ParticleSystem3`) false)
      (`KismetSystemLibrary.Delay` 0.1)
      (`ActorComponent.Activate` (`self.P_Explosion05`) false)
      (`ActorComponent.Activate` (`self.S_Explosion05`) false)
      (`KismetSystemLibrary.Delay` 0.1)
      (`ActorComponent.Activate` (`self.ParticleSystem5`) false)
      (`ActorComponent.Activate` (`self.Audio5`) false)
      (goto _label))
    (:`then_1`
      (`KismetSystemLibrary.Delay` 0.05)
      (`ActorComponent.Activate` (`self.P_Explosion01`) false)
      (`ActorComponent.Activate` (`self.S_Explosion01`) false)
      (`KismetSystemLibrary.Delay` 0.1)
      (`ActorComponent.Activate` (`self.Audio1`) false)
      (`ActorComponent.Activate` (`self.ParticleSystem1`) false)
      (`KismetSystemLibrary.Delay` 0.1)
      (`ActorComponent.Activate` (`self.ParticleSystem2`) false)
      (`ActorComponent.Activate` (`self.Audio2`) false)
      (`KismetSystemLibrary.Delay` 0.1)
      (`ActorComponent.Activate` (`self.P_Explosion04`) false)
      (`ActorComponent.Activate` (`self.S_Explosion04`) false)
      (`KismetSystemLibrary.Delay` 0.1)
      (`ActorComponent.Activate` (`self.Audio4`) false)
      (`ActorComponent.Activate` (`self.ParticleSystem4`) false)
      (`KismetSystemLibrary.Delay` 0.1)
      (`ActorComponent.Activate` (`self.P_Explosion06`) false)
      (`ActorComponent.Activate` (`self.S_Explosion06`) false)
      (goto _label))))

(fn `UserConstructionScript`)